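; Game mode that owns the game's UI flow: HUD, inventory, pause and end screens.
; On BeginPlay it sets game-only input, creates the HUD and inventory widgets and passes them references to itself, plus the AwooCharacter for the inventory.
; Tick runs the character's item trace and polls its pause flag.
; Pause, inventory and end-game events show their widgets, pause the game and reveal the cursor.
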(event `self.ReceiveBeginPlay`
  (bind _returnvalue (`GameplayStatics.GetPlayerController` 0))
  (bind _myinvhud (`self.myInvHUD`))
  ;[1 1 1] input controls
  (`WidgetBlueprintLibrary.SetInputMode_GameOnly` _returnvalue)
  (set `PlayerController.bShowMouseCursor` false _returnvalue)
  ;[1 1 1] create in game HUD
  (bind _returnvalue_2 (`|CreateWidget` "/Game/myBlueprint/BP_MyHUD.BP_MyHUD_C"))
  (bind _output_get (set `self.GameHUD` _returnvalue_2))
  (`UserWidget.AddToViewport` _output_get 0)
  ;[1 1 1] create inventory
  (bind _returnvalue_3 (`|CreateWidget` "/Game/myBlueprint/BP_InventoryHUD.BP_InventoryHUD_C"))
  (set `self.myInvHUD` _returnvalue_3)
  ;[1 1 1] init variables
  (bind _asawoo_character (cast `AwooCharacter` (`GameplayStatics.GetPlayerCharacter` 0)))
  (set `self.GameChar` _asawoo_character)
  (set `/Game/myBlueprint/BP_MyHUD.HUDGameMode` self (`self.GameHUD`))
  (set `/Game/myBlueprint/BP_InventoryHUD.invGameMode` self _myinvhud)
  (set `/Game/myBlueprint/BP_InventoryHUD.invGameChar` (`self.GameChar`) _myinvhud))

(event `self.ReceiveTick`
  (params (DeltaSeconds :type "Float (single-precision)"))
  (bind _gamechar (`self.GameChar`))
  ;[1 1 1] check for item
  (`AwooCharacter.CallMyTrace` _gamechar)
  ;[1 1 1] check if paused
  (if (`AwooCharacter.PausePressed` _gamechar)
    (`self.pauseGame`)))

(event `endGame`
  (params (IsPlayerWin :type Boolean))
  ;[1 1 1] end game event
  (bind _returnvalue (`|CreateWidget` "/Game/myBlueprint/BP_EndHUD.BP_EndHUD_C"))
  (bind _output_get (set `self.EndRef` _returnvalue))
  (`GameplayStatics.SetGamePaused` true)
  (set `/Game/myBlueprint/BP_EndHUD.isVictory` IsPlayerWin (`self.EndRef`))
  (`UserWidget.AddToViewport` _output_get 0)
  (set `PlayerController.bShowMouseCursor` true (`GameplayStatics.GetPlayerController` 0)))

(event `endScreen`
  ;[1 1 1] end game event
)

(event `pauseGame`
  (bind _returnvalue (`GameplayStatics.GetPlayerController` 0))
  ;[1 1 1] pause game event
  (`/Engine/EditorBlueprintResources/StandardMacros.IsValid` (`self.PauseRef`)
    (:`Is Valid`
      _)
    (:`Is Not Valid`
      ;;[1 1 1] create widget if not valid
      (bind _returnvalue_2 (`|CreateWidget` "/Game/myBlueprint/BP_PauseHUD.BP_PauseHUD_C"))
      (bind _output_get (set `self.PauseRef` _returnvalue_2))))
  ;;[1 1 1] player control
  (set `PlayerController.bShowMouseCursor` true _returnvalue)
  (`WidgetBlueprintLibrary.SetInputMode_UIOnlyEx` _returnvalue _output_get)
  ;;[1 1 1] add HUD
  (`UserWidget.AddToViewport` (`self.PauseRef`) 0)
  (`GameplayStatics.SetGamePaused` true)
  (set `AwooCharacter.PausePressed` false (`self.GameChar`)))

(event `OpenInventory`
  (bind _returnvalue (`GameplayStatics.GetPlayerController` 0))
  ;[1 1 1] openInventory
  (set `PlayerController.bShowMouseCursor` true _returnvalue)
  (`WidgetBlueprintLibrary.SetInputMode_UIOnlyEx` _returnvalue (`self.myInvHUD`))
  (`UserWidget.AddToViewport` (`self.myInvHUD`) 0)
  (`GameplayStatics.SetGamePaused` true))

(fn `UserConstructionScript`)