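; BP_Laser is a rotating laser hazard that damages any AwooCharacter its beam hits.
; Each tick it line traces forward on the Camera channel, ends the Niagara beam at the hit or maximum distance, and shows the impact effect on hits.
; It yaws by RotateSpeed scaled with delta time, while damage is a fixed amount per frame.
; BeginPlay tints both effects red, and the trace's debug line is drawn each frame.
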(event `self.ReceiveBeginPlay`
  (`FXSystemComponent.SetColorParameter` (`self.NLaser`) "Color" (struct :`R` 1.0 :`B` 0.08466 :`A` 1.0))
  (`FXSystemComponent.SetColorParameter` (`self.NLaserImpact`) "Color" (struct :`R` 1.0 :`B` 0.08466 :`A` 1.0)))

(event `self.ReceiveTick`
  (params (DeltaSeconds :type "Float (single-precision)"))
  (bind _returnvalue (`self.K2_GetActorLocation`))
  (bind _nlaserimpact (`self.NLaserImpact`))
  (set `self.DeltaTime` DeltaSeconds)
  (bind _output_get (set `self.TraceEnd` (+ _returnvalue (* (`self.GetActorForwardVector`) (`self.distance`)))))
  (bind _outhit (`KismetSystemLibrary.LineTraceSingle` :`Start` _returnvalue :`End` _output_get :`TraceChannel` "TraceTypeQuery2" :`DrawDebugType` "ForOneFrame"))
  (bind (_bblockinghit _binitialoverlap _time _distance _location _impactpoint _normal _impactnormal _physmat _hitactor) (`GameplayStatics.BreakHitResult` _outhit))
  (set `self.Hit` _bblockinghit)
  (set `self.HitLoc` _location)
  (`FXSystemComponent.SetVectorParameter` (`self.NLaser`) "LaserEnd" (`KismetMathLibrary.SelectVector` (`self.HitLoc`) (`self.TraceEnd`) (`self.Hit`)))
  (`SceneComponent.SetVisibility` _nlaserimpact (`self.Hit`) false)
  (`SceneComponent.K2_SetWorldLocation` _nlaserimpact (`self.HitLoc`) false false)
  (`self.K2_AddActorLocalRotation` (`KismetMathLibrary.MakeRotator` 0.0 0.0 (* (`self.RotateSpeed`) (`self.DeltaTime`))))
  (bind _asawoo_character (cast `AwooCharacter` _hitactor))
  (`AwooCharacter.ReceiveDamage` _asawoo_character 0.3))

(fn `UserConstructionScript`)